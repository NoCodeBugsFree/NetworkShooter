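; BP_Shotgun is a child weapon Blueprint that adds the shotgun's firing effects by extending the parent's PlayWeaponFX event.
; A single camera-origin line trace along the shoot direction places a timed bullet-hole decal on a hit and spawns a BP_Trail from the muzzle toward it.
; It also attaches a muzzle flash and, unless IsOtherPlayer, runs a timeline that applies recoil through the owner's controller pitch.
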(event `self.PlayWeaponFX`
  (bind _returnvalue_location (`KismetMathLibrary.BreakTransform` (`SceneComponent.GetSocketTransform` (`self.GunMesh`) "Muzzle" "RTS_World")))
  (`parent.PlayWeaponFX`)
  (`|ExecutionSequence`
    (:`then_0`
      ;[0.02493 1 0 0.5] Decal
      (bind _weaponowner (`self.WeaponOwner`)
        (:`then`
          (bind _returnvalue (`SceneComponent.K2_GetComponentLocation` (`PCh.CameraComponent` _weaponowner)))
          (bind (_outhit _returnvalue_2) (`KismetSystemLibrary.LineTraceSingleForObjects` _returnvalue (+ _returnvalue (* (`self.GetShootDirection`) (`self.ShootDistance`))) (`|MakeArray` "ObjectTypeQuery3" "ObjectTypeQuery1" "ObjectTypeQuery2" "ObjectTypeQuery4" :!type "EObjectTypeQuery Enum") false (`|MakeArray` self (`self.GetInstigator`) :!type "Actor Object Reference") "None" true (struct :`R` 0.117122 :`B` 0.5 :`A` 1.0) (struct :`G` 0.167679 :`B` 1.0 :`A` 1.0)))
          (if _returnvalue_2
            (bind (_bblockinghit _binitialoverlap _time _distance _location _impactpoint _normal) (`GameplayStatics.BreakHitResult` _outhit))
            (bind _returnvalue_3 (`|SpawnActorFromClass` "/Script/Engine.DecalActor" (`KismetMathLibrary.MakeTransform` _location (struct) (0.02 0.02 0.02)) "AlwaysSpawn" "OverrideRootScale" null null))
            (`self.SetLifeSpan` _returnvalue_3 30.0)
            (`DecalComponent.SetDecalMaterial` (`DecalActor.Decal` _returnvalue_3) (`self.HoleMaterial`))
            (`self.K2_SetActorRotation` _returnvalue_3 (`KismetMathLibrary.Conv_VectorToRotator` (* _normal -1.0)) false)
            (`DecalComponent.SetFadeScreenSize` (`DecalActor.Decal` _returnvalue_3) 0.001)
            (bind (_bblockinghit_2 _binitialoverlap_2 _time_2 _distance_2 _location_2 _impactpoint_2 _normal_2 _impactnormal _physmat _hitactor _hitcomponent _hitbonename _hititem _faceindex _tracestart _traceend) (`GameplayStatics.BreakHitResult` _outhit))
            ;[0.02493 1 0 0.5] Bullet Trail FX
            (`|SpawnActorFromClass` "/Game/BP/Weapons/Trail/BP_Trail.BP_Trail_C" (`KismetMathLibrary.MakeTransform` _returnvalue_location (`KismetMathLibrary.FindLookAtRotation` _returnvalue_location (`KismetMathLibrary.SelectVector` _location_2 _traceend _bblockinghit_2))) "AlwaysSpawn" "OverrideRootScale" null _outhit null)))
        (:`else`)))
    (:`then_1`
      ;[0.02493 1 0 0.5] muzzle flash
      (`GameplayStatics.SpawnEmitterAttached` "/Game/FX/P_MuzzleFlash.P_MuzzleFlash" (`self.GunMesh`) "Muzzle" (0.0 0.0 0.0) (struct) (1.0 1.0 1.0) "SnapToTarget"))
    (:`then_2`
      ;[0.02493 1 0 0.5] recoil anim
      (if (not (`/Game/BP/Weapons/BP_Weapon.IsOtherPlayer`))
        (bind (_direction _lerp) (`Timeline|Timeline_0` :!via `PlayFromStart`)
          (:`Update`
            (bind _weaponowner_2 (`self.WeaponOwner`)
              (:`then`
                (`Pawn.AddControllerPitchInput` _weaponowner_2 (* _lerp (`self.Recoil`) -1.0)))
              (:`else`))))))))

(fn `UserConstructionScript`
  (`parent.UserConstructionScript`))