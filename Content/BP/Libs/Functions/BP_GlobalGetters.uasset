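; Blueprint function library of global getters that return the game's framework objects already cast to project classes.
; Game mode getters cast the current game mode to the base, team or deathmatch Blueprint class.
; Player state getters take a controller and cast its PlayerState to the base or team player state class.
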(fn `GetDeathmathGM`
  (returns (`AsBP Death Match GM` :type "/Game/BP/Game/BP_DeathMatchGM Object Reference"))
  (return (cast `/Game/BP/Game/BP_DeathMatchGM` (`GameplayStatics.GetGameMode` null) :!pure true)))

(fn `GetGM`
  (returns (`AsBP GM` :type "/Game/BP/Game/BP_GM Object Reference"))
  (return (cast `/Game/BP/Game/BP_GM` (`GameplayStatics.GetGameMode` null) :!pure true)))

(fn `GetPlayerStateByController`
  (params (Controller :type "Controller Object Reference"))
  (returns (`AsBP PS` :type "/Game/BP/Player/BP_PS Object Reference"))
  (return (cast `/Game/BP/Player/BP_PS` (`Controller.PlayerState` Controller) :!pure true)))

(fn `GetTeamGM`
  (returns (`AsBP Team GM` :type "/Game/BP/Game/BP_TeamGM Object Reference"))
  (return (cast `/Game/BP/Game/BP_TeamGM` (`GameplayStatics.GetGameMode` null) :!pure true)))

(fn `GetTeamPlayerStateByController`
  (params (Controller :type "Controller Object Reference"))
  (returns (`AsBP Team PS` :type "/Game/BP/Player/BP_TeamPS Object Reference"))
  (return (cast `/Game/BP/Player/BP_TeamPS` (`Controller.PlayerState` Controller) :!pure true)))